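; Trigger actor that switches the player ship to a new perspective, passing along new stage music and a new track.
; When the tagged player overlaps it, it either switches at once or first rotates the ship along a timeline.
; The target rotation is either the Arrow's world rotation (absolute) or an offset from the ship's current rotation (relative).
; A text label shows the target perspective; the track-detach event is never run.
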(event `self.ReceiveBeginPlay`
  ;[1 1 1] Save Player reference
  (bind _asbp_player_ship (cast `/Game/ASST/Blueprints/Characters/Player/BP_PlayerShip` (`GameplayStatics.GetPlayerPawn` 0)))
  (set `self.PlayerRef` _asbp_player_ship))

(event `self.Trigger.OnComponentBeginOverlap`
  (params (OverlappedComponent :type "PrimitiveComponent Object Reference") (OtherActor :type "Actor Object Reference") (OtherComp :type "PrimitiveComponent Object Reference") (OtherBodyIndex :type Integer) (bFromSweep :type Boolean) (SweepResult :type "HitResult Structure (by ref)"))
  ;[1 1 1] Overlap only Player
  (if (`self.ActorHasTag` OtherActor "Player")
    (if (`self.RotatePlayer?`)
      (`self.EventRotatePlayer`)
      (else
        (`self.Event Switch Perspective`)))))

(event `EventRotatePlayer`
  ;[1 1 1] CUSTOM EVENTS
  (set `self.InitPlayerRotation` (`self.K2_GetActorRotation` (`self.PlayerRef`)))
  (switch `/Game/ASST/Enums/Enum_StageClear_RotationType` (`self.RotationType`)
    (:`NewEnumerator0`
      (`self.fnCalculateAbsoluteRotation`)
      (bind (_direction _alpha) (`Timeline|TM_RotatePlayer` :!label _label)
        (:`Update`
          (`self.K2_SetActorRotation` (`self.PlayerRef`) (`KismetMathLibrary.RLerp` (`self.InitPlayerRotation`) (`self.NewRotation`) _alpha true) false))
        (:`Finished`
          (`self.Event Switch Perspective`))))
    (:`NewEnumerator1`
      (`self.fnCalculateDeltaRotation`)
      (goto _label))))

(event `EventCheckGameMode`
  ;[1 1 1] CUSTOM EVENTS
  (if (`/Game/ASST/Blueprints/Characters/Player/BP_PlayerShip.TrackModeActive` (`self.PlayerRef`))
    (set `/Game/ASST/Blueprints/Characters/Player/BP_PlayerShip.FollowTrack?` false (`self.PlayerRef`))
    (set `/Game/ASST/Blueprints/Characters/Player/BP_PlayerShip.TrackFinished?` true (`self.PlayerRef`))
    (`KismetSystemLibrary.Delay` 0.1)))

(event `Event Switch Perspective`
  ;[1 1 1] CUSTOM EVENTS
  (`/Game/ASST/Blueprints/Characters/Player/BP_PlayerShip.Event Switch Persepctive` (`self.PlayerRef`) (`self.NewPersepctiveMusic`) (`self.NewPerspective`) (`self.NewTrack`)))

(fn `fnCalculateAbsoluteRotation`
  ;[1 1 1] Set new rotation to the Arrow's world rotation
  (set `self.NewRotation` (`SceneComponent.K2_GetComponentRotation` (`self.Arrow`))))

(fn `fnCalculateDeltaRotation`
  (bind _newrotation_roll (`KismetMathLibrary.BreakRotator` (`self.NewRotation`)))
  (bind _initplayerrotation_roll (`KismetMathLibrary.BreakRotator` (`self.InitPlayerRotation`)))
  (bind (_newrotation_roll_2 _newrotation_pitch) (`KismetMathLibrary.BreakRotator` (`self.NewRotation`)))
  (bind (_initplayerrotation_roll_2 _initplayerrotation_pitch) (`KismetMathLibrary.BreakRotator` (`self.InitPlayerRotation`)))
  (bind (_initplayerrotation_roll_3 _initplayerrotation_pitch_2 _initplayerrotation_yaw) (`KismetMathLibrary.BreakRotator` (`self.InitPlayerRotation`)))
  (bind (_newrotation_roll_3 _newrotation_pitch_2 _newrotation_yaw) (`KismetMathLibrary.BreakRotator` (`self.NewRotation`)))
  ;[1 1 1] Set new rotation to current rotation + delta rotation
  (set `self.NewRotation` (`KismetMathLibrary.MakeRotator` (+ _initplayerrotation_roll _newrotation_roll) (+ _initplayerrotation_pitch _newrotation_pitch) (+ _initplayerrotation_yaw _newrotation_yaw))))

(fn `UserConstructionScript`
  (`TextRenderComponent.K2_SetText` (`self.TextRender`) (`KismetTextLibrary.Conv_StringToText` (`KismetStringLibrary.Concat_StrStr` "Switch To: " (`|GetEnumeratorNameAsString` (cast `/Game/ASST/Enums/Enum_PerspectiveTypes` (`self.NewPerspective`)))))))