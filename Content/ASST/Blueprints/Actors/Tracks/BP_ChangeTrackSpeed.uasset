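; Track trigger actor that changes the player ship's track speeds when the ship first overlaps it.
; A one-shot overlap starts a timeline whose alpha scales the configured forward speed into the ship's base track speed.
; It also updates current speed, or braking speed while braking, plus horizontal and vertical speeds; boosting without braking leaves these untouched.
; The construction script displays the forward speed on a text render.
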(event `self.Trigger.OnComponentBeginOverlap`
  (params (OverlappedComponent :type "PrimitiveComponent Object Reference") (OtherActor :type "Actor Object Reference") (OtherComp :type "PrimitiveComponent Object Reference") (OtherBodyIndex :type Integer) (bFromSweep :type Boolean) (SweepResult :type "HitResult Structure (by ref)"))
  ;[1 1 1] Only overlap Player
  (if (`self.ActorHasTag` OtherActor "Player")
    (bind _asbp_player_ship (cast `/Game/ASST/Blueprints/Characters/Player/BP_PlayerShip` OtherActor))
    (set `self.PlayerRef` _asbp_player_ship)
    (`/Engine/EditorBlueprintResources/StandardMacros.DoOnce` false
      (:`Completed`
        (`self.EventSetNewSpeed`)))))

(event `EventSetNewSpeed`
  (bind _playerref (`self.PlayerRef`))
  (bind (_direction _alpha) (`Timeline|TMSetSpeed`)
    (:`Update`
      (set `self.SmoothForwardSpeed` (* _alpha (`self.ForwardSpeed`)))
      ;[1 1 1] Set the TrackSpeed, CurrentTrackSpeed and BrakingTrackSpeed to the new value
      (set `/Game/ASST/Blueprints/Characters/Player/BP_PlayerShip.ThisTrackSpeed` (`self.SmoothForwardSpeed`) (`self.PlayerRef`))
      ;;[1 1 1] If Player is NOT boosting or braking, set CurrentTrackSpeed to NewSpeed
      (if (not (or (`/Game/ASST/Blueprints/Characters/Player/BP_PlayerShip.Braking` _playerref) (`/Game/ASST/Blueprints/Characters/Player/BP_PlayerShip.Boosting` _playerref)))
        ;;[1 1 1] Change track speed to NewSpeed
        (set `/Game/ASST/Blueprints/Characters/Player/BP_PlayerShip.CurrentTrackSpeed` (`self.SmoothForwardSpeed`) (`self.PlayerRef`))
        ;[1 1 1] Set the new horizontal and vertical track speeds
        (set `/Game/ASST/Blueprints/Characters/Player/BP_PlayerShip.HorizontalTrackSpeed` (`self.HorizontalSpeed`) (`self.PlayerRef`) :!label _label)
        (set `/Game/ASST/Blueprints/Characters/Player/BP_PlayerShip.VerticalTrackSpeed` (`self.VerticalSpeed`) (`self.PlayerRef`))
        (else
          ;;[1 1 1] If Player is braking, set the BrakingTrackSpeed to NewSpeed
          (if (`/Game/ASST/Blueprints/Characters/Player/BP_PlayerShip.Braking` (`self.PlayerRef`))
            (set `/Game/ASST/Blueprints/Characters/Player/BP_PlayerShip.BrakingTrackSpeed` (`self.SmoothForwardSpeed`) (`self.PlayerRef`))
            (goto _label)))))))

(fn `UserConstructionScript`
  (`TextRenderComponent.K2_SetText` (`self.RenderSpeed`) (`KismetTextLibrary.Conv_DoubleToText` (`self.ForwardSpeed`) "HalfToEven")))