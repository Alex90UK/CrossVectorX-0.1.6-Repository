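; BP_Laser is a laser projectile actor that ignores the player pawn and damages what it hits.
; The construction script sets velocity and tags, and BeginPlay sets the lifespan and enables homing on a valid Target, with stronger acceleration for distant targets.
; Collision hits on actors without the Player tag send a damage message with hit info, spawn explosion particles and sound, then destroy the laser after a short delay.
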(event `self.ReceiveBeginPlay`
  (bind _target (`self.Target`))
  (bind _projectilemovement (`self.ProjectileMovement`))
  ;[1 1 1] Set Laser lifespan
  (`self.SetLifeSpan` (`self.TimeToLive`))
  ;[1 1 1] Ignore player pawn
  (`PrimitiveComponent.IgnoreActorWhenMoving` (`self.LaserMesh`) (`GameplayStatics.GetPlayerPawn` 0) true)
  ;[1 1 1] Add slight homing
  (`/Engine/EditorBlueprintResources/StandardMacros.IsValid` _target
    (:`Is Valid`
      (if (>= (`KismetMathLibrary.VSize` (- (`self.K2_GetActorLocation` _target) (`self.K2_GetActorLocation`))) 10000.0)
        (set `ProjectileMovementComponent.HomingAccelerationMagnitude` 800.0 _projectilemovement)
        (else
          (set `ProjectileMovementComponent.HomingAccelerationMagnitude` 450.0 _projectilemovement)))
      (set `ProjectileMovementComponent.HomingTargetComponent` (`Actor.RootComponent` _target) _projectilemovement)
      (set `ProjectileMovementComponent.bIsHomingProjectile` true _projectilemovement))))

(event `self.LaserMesh.OnComponentHit`
  (params (HitComponent :type "PrimitiveComponent Object Reference") (OtherActor :type "Actor Object Reference") (OtherComp :type "PrimitiveComponent Object Reference") (NormalImpulse :type "Vector Structure") (Hit :type "HitResult Structure (by ref)")))

(event `self.Collision.OnComponentHit`
  (params (HitComponent :type "PrimitiveComponent Object Reference") (OtherActor :type "Actor Object Reference") (OtherComp :type "PrimitiveComponent Object Reference") (NormalImpulse :type "Vector Structure") (Hit :type "HitResult Structure (by ref)"))
  (bind _returnvalue (`SceneComponent.K2_GetComponentLocation` (`self.HitComponent`)))
  (set `self.HitComponent` HitComponent)
  (set `self.OtherActor` OtherActor)
  ;[1 1 1] Do not hit the Player
  (if (not (`self.ActorHasTag` (`self.OtherActor`) "Player"))
    ;[1 1 1] Apply point damage
    (message `/Game/ASST/Blueprints/Actors/Interfaces/IDamage.CauseDamage` (`self.OtherActor`) (`KismetMathLibrary.FTrunc` (`self.BaseDamage`)) self Hit (`self.EventName`) (* (`.ImpactNormal` (`GameplayStatics.BreakHitResult` Hit)) -1.0))
    ;[1 1 1] Spawn emitter at hit location
    (`GameplayStatics.SpawnEmitterAtLocation` (`self.ExplosionParticles`) _returnvalue)
    ;[1 1 1] Play explosion sound
    (`GameplayStatics.PlaySoundAtLocation` (`self.ExplosionSound`) _returnvalue)
    ;[1 1 1] Wait for 0.2secs and destroy the actor
    (`KismetSystemLibrary.Delay` 0.1)
    (`self.K2_DestroyActor`)))

(fn `UserConstructionScript`
  ;[1 1 1] Set velocity
  (set `MovementComponent.Velocity` (`self.ProjectileVelocity`) (`self.ProjectileMovement`))
  ;[1 1 1] Set actor tags
  (set `self.Tags` (`self.ActorTags`)))