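; BP_Utility is a base Blueprint for player ship utilities with a cooldown-gated Fire.
; It caches the player ship on BeginPlay; Fire runs UtilityFunctionality when off cooldown, then starts a timer that calls EndcoolDown to clear the lock.
; UtilityFunctionality is an empty hook, apparently for child classes to override.
; ModifyUtilityLevel switches on a level modifier but has no branch logic.
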(event `self.ReceiveBeginPlay`
  ;[1 1 1] Begin play
  (set `self.PlayerRef` (cast `/Game/ASST/Blueprints/Characters/Player/BP_PlayerShip` (`GameplayStatics.GetPlayerPawn` 0) :!pure true)))

(fn `CoolDown`
  (bind _returnvalue (`KismetSystemLibrary.K2_SetTimer` null "EndcoolDown" (`self.CoolDownTime`)))
  (set `self.CooldownTimer` _returnvalue))

(fn `EndcoolDown`
  (set `self.OnCoolDown` false))

(fn `Fire`
  (if (not (`self.OnCoolDown`))
    (set `self.OnCoolDown` true)
    (`self.UtilityFunctionality`)
    (`self.CoolDown`)))

(fn `ModifyUtilityLevel`
  (params (ModifyWeaponLevel :type Integer))
  (switch `int` ModifyWeaponLevel))

(fn `UserConstructionScript`)

(fn `UtilityFunctionality`)