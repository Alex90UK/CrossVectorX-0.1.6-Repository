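; Base player ship weapon with auto-fire and charge-shot modes, leaving basic fire and level changes as empty stubs.
; Fire starts a looping timer that either calls FireBasic or builds clamped charge.
; On release, charged shots can require a minimum charge, with insufficient charge draining on another timer.
; AttachToPlayer snaps the weapon to the player ship and moves fire points to enum-named ship sockets.
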(event `self.ReceiveBeginPlay`
  ;[1 1 1] Begin play
  (set `self.PlayerRef` (cast `/Game/ASST/Blueprints/Characters/Player/BP_PlayerShip` (`GameplayStatics.GetPlayerPawn` 0) :!pure true)))

(event `StopFiring`
  ;[1 1 1] Stop firing auto
  (`KismetSystemLibrary.K2_ClearAndInvalidateTimerHandle` (`self.FireRateTimer`))
  (`KismetSystemLibrary.K2_ClearAndInvalidateTimerHandle` (`self.Chargetimer`))
  (`self.Shoot_Charged`))

(event `Fire`
  (if (`self.IsAuto`)
    ;[1 1 1] Auto Fire
    (bind _returnvalue (`KismetSystemLibrary.K2_SetTimerDelegate` (delegate `Shoot`) (`self.FireRate`) true))
    (set `self.FireRateTimer` _returnvalue)
    (else
      ;[1 1 1] Charge Weapon
      (if (`self.IsChargeWeapon`)
        (`KismetSystemLibrary.K2_ClearAndInvalidateTimerHandle` (`self.UnchargeTimer`))
        (bind _returnvalue_2 (`KismetSystemLibrary.K2_SetTimerDelegate` (delegate `ChargeWeapon`) (`self.ChargeTime`) true))
        (set `self.Chargetimer` _returnvalue_2)))))

(event `Shoot`
  ;[1 1 1] Auto Fire
  (`self.Fire_Basic`))

(event `UnchargeWeapon`
  ;[1 1 1] Charge Weapon
  (bind _returnvalue (`KismetSystemLibrary.K2_SetTimerDelegate` (delegate `Uncharge`) (`self.ChargeTime`) true))
  (set `self.UnchargeTimer` _returnvalue))

(event `Uncharge`
  ;[1 1 1] Charge Weapon
  (set `self.CurrentCharge` (`KismetMathLibrary.FClamp` (- (`self.CurrentCharge`) (`self.ChargeAmount`)) 0.0 (`self.MaxCharge`)))
  (if (<= (`self.CurrentCharge`) 0.0)
    (`KismetSystemLibrary.K2_ClearAndInvalidateTimerHandle` (`self.UnchargeTimer`))))

(event `ChargeWeapon`
  ;[1 1 1] Charge Weapon
  (set `self.CurrentCharge` (`KismetMathLibrary.FClamp` (+ (`self.CurrentCharge`) (`self.ChargeAmount`)) 0.0 (`self.MaxCharge`)))
  (if (>= (`self.CurrentCharge`) (`self.MaxCharge`))
    (`KismetSystemLibrary.K2_ClearAndInvalidateTimerHandle` (`self.Chargetimer`))))

(event `Shoot_Charged`
  ;[1 1 1] ShootCharge
  (if (`self.RequireMinCharge`)
    (if (>= (`self.CurrentCharge`) (`self.MinCharge`))
      (`self.Fire_Charged`)
      (set `self.CurrentCharge` 0.0 :!label _label)
      (else
        (`self.UnchargeWeapon`)))
    (elif (!= (`self.ChargeAmount`) 0.0)
      (`self.Fire_Charged`)
      (goto _label))))

(fn `AttachToPlayer`
  (locals (FirePoints :type "Array of StaticMeshComponent Object Reference"))
  (`self.K2_AttachToActor` self (`self.PlayerRef`) "None" "SnapToTarget" "SnapToTarget" "SnapToTarget" true)
  (`self.MoveFirepointsToSockets` (`/Game/ASST/Blueprints/Characters/Player/BP_PlayerShip.Ship` (`self.PlayerRef`)) (`self.Sockets`) (`|MakeArray` (`self.FirePointMesh`) (`self.FirePointMesh2`)) (`self.ESockets`)))

(fn `Fire_Basic`)

(fn `Fire_Charged`
  (returns (Return :type Boolean))
  (set `self.CurrentCharge` 0.0)
  (return false))

(fn `ModifyWeaponLevel`
  (params (NewLevel :type Integer))
  (switch `int` NewLevel))

(fn `MoveFirepointsToSockets`
  (params (ShipComponentRef :type "SceneComponent Object Reference") (Sockets :type "Array of Name") (FirePoints :type "Array of StaticMeshComponent Object Reference") (ESockets :type "Array of /Game/ASST/Blueprints/Actors/Weapons/Player/Enum_LoadoutSocketLoc Enum" :default _))
  (returns (Return :type Boolean))
  (for (_array_element _array_index) ESockets
    (bind _output (`|GetArrayItem` FirePoints _array_index))
    (`/Engine/EditorBlueprintResources/StandardMacros.IsValid` _output
      (:`Is Valid`
        (bind _returnvalue_location (`KismetMathLibrary.BreakTransform` (`SceneComponent.GetSocketTransform` ShipComponentRef (`KismetStringLibrary.Conv_StringToName` (`|GetEnumeratorNameAsString` _array_element)) "RTS_Component")))
        (`SceneComponent.K2_SetRelativeLocation` _output _returnvalue_location false true)))))

(fn `UserConstructionScript`)