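; Spring-arm camera actor that follows BP_PlayerShip, registers itself with the player on Init and can become the view target.
; Tick dispatches by camera mode: All Range copies the ship's transform, Track rides the track spline with scaled panning, Stage Clear plays a timeline orbit and close-up.
; Somersaults inherit roll in All Range and use look-at in Track, as does player death.
; Perspective switches re-pose the arm for top-down, side-on or third-person.
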(event `self.ReceiveBeginPlay`)

(event `/Game/ASST/Blueprints/Characters/Player/ISetup.Init`
  (bind _playerref (`self.PlayerRef`))
  ;[1 1 1] Save the Player reference
  (bind _asbp_player_ship (cast `/Game/ASST/Blueprints/Characters/Player/BP_PlayerShip` (`GameplayStatics.GetPlayerPawn` 0)))
  (bind _output_get (set `self.PlayerRef` _asbp_player_ship))
  ;[1 1 1] Check if Player reference is valid
  (if (`KismetSystemLibrary.IsValid` _output_get)
    ;[1 1 1] Set Initial TargetLocation
    (set `self.TargetLocation` (`self.K2_GetActorLocation` (`self.PlayerRef`)))
    ;[1 1 1] Set Initial TargetRotation
    (set `self.TargetRotation` (`self.K2_GetActorRotation` (`self.PlayerRef`)))
    ;[1 1 1] Save the Max Z and Y values from Player
    (set `self.MaxZValue` (`/Game/ASST/Blueprints/Characters/Player/BP_PlayerShip.MaxZValue` _playerref))
    (set `self.MaxYValue` (`/Game/ASST/Blueprints/Characters/Player/BP_PlayerShip.MaxYValue` _playerref))
    ;[1 1 1] Set CameraActorRef to Self
    (set `/Game/ASST/Blueprints/Characters/Player/BP_PlayerShip.FixedCameraActorRef` self (`self.PlayerRef`))
    ;[1 1 1] If this actor is active, set ViewTarget to self
    (if (`/Game/ASST/Blueprints/Characters/Player/BP_PlayerShip.FixedCameraActive?` (`self.PlayerRef`))
      ;[1 1 1] Automatically set this camera as active
      (`PlayerController.SetViewTargetWithBlend` (`GameplayStatics.GetPlayerController` 0) self 0.0 "VTBlend_Cubic" 0.0 false))))

(event `self.ReceiveTick`
  (params (DeltaSeconds :type "Float (single-precision)"))
  ;[1 1 1] Check Player reference is valid
  (if (`KismetSystemLibrary.IsValid` (`self.PlayerRef`))
    ;[1 1 1] Check if Player is NOT dead
    (if (not (`/Game/ASST/Blueprints/Characters/Player/BP_PlayerShip.IsDead` (`self.PlayerRef`)))
      ;[1 1 1] Track player by using the appropriate method
      (switch `/Game/ASST/Enums/Enum_CameraMode` (`self.CameraMode`)
        (:`NewEnumerator0`
          (`self.EventAllRangeMode`))
        (:`NewEnumerator1`
          (if (not (`self.IsSwitching`))
            (`self.EventTrackMode`)))
        (:`NewEnumerator2`
          (`self.EventStageClear`)))
      (else
        ;[1 1 1] Player is dead - keep the camera in the same location but follow player
        (`self.K2_SetActorRotation` (`KismetMathLibrary.FindLookAtRotation` (`self.K2_GetActorLocation`) (`self.K2_GetActorLocation` (`self.PlayerRef`))))))))

(event `SwitchCameraPersepctive`
  (params (Persepctive :type "/Game/ASST/Enums/Enum_PerspectiveTypes Enum" :default "NewEnumerator0"))
  ;[1 1 1] Switch perspective
  (set `self.CurrentPerspective` Persepctive)
  (set `self.IsSwitching` true)
  (switch `/Game/ASST/Enums/Enum_PerspectiveTypes` (`self.CurrentPerspective`)
    (:`NewEnumerator0`
      (`self.RelativeSpringArm_CameraTransformOffset` (struct :`Pitch` -90.0) 2800.0))
    (:`NewEnumerator1`
      (`self.RelativeSpringArm_CameraTransformOffset` (struct :`Pitch` -90.0 :`Roll` -90.0) 2200.0 (0.0 0.0 0.0) (struct :`Roll` 90.0)))
    (:`NewEnumerator2`
      (`self.RelativeSpringArm_CameraTransformOffset` (struct) 600.0 (0.0 0.0 0.0) (struct :`Pitch` -10.0))))
  (set `self.IsSwitching` false))

(event `EventAllRangeMode`
  (bind _playerref (`self.PlayerRef`))
  (bind _playerref_2 (`self.PlayerRef`))
  ;[1 1 1] CUSTOM EVENTS
  (`SceneComponent.K2_SetRelativeLocation` (`self.Camera_3D`) (`KismetMathLibrary.MakeVector` 0.0 0.0 (`self.CameraZOffset`)) false true)
  (`self.K2_SetActorLocationAndRotation` (`self.K2_GetActorLocation` _playerref) (`self.K2_GetActorRotation` _playerref) false true)
  (if (or (`/Game/ASST/Blueprints/Characters/Player/BP_PlayerShip.DoingSomersault?` _playerref_2) (`/Game/ASST/Blueprints/Characters/Player/BP_PlayerShip.DoingUTurn?` _playerref_2))
    (`|ExecutionSequence`
      (:`then_0`
        (`/Engine/EditorBlueprintResources/StandardMacros.DoOnce` false :!label _label
          (:`Completed`
            (set `SpringArmComponent.bInheritRoll` true (`self.SpringArm_3D`))
            (set `SpringArmComponent.bEnableCameraRotationLag` false (`self.SpringArm_3D`)))))
      (:`then_1`
        (goto _label_2 :!via `Reset`)))
    (else
      (`|ExecutionSequence`
        (:`then_0`
          (`/Engine/EditorBlueprintResources/StandardMacros.DoOnce` false :!label _label_2
            (:`Completed`
              (set `SpringArmComponent.bInheritRoll` false (`self.SpringArm_3D`))
              (set `SpringArmComponent.bEnableCameraRotationLag` true (`self.SpringArm_3D`)))))
        (:`then_1`
          (goto _label :!via `Reset`))))))

(event `EventTrackMode`
  (bind _playerref (`self.PlayerRef`))
  (bind _camerapercentoffset (`self.CameraPercentOffset`))
  (bind _playerref_2 (`self.PlayerRef`))
  (bind _returnvalue_roll (`KismetMathLibrary.BreakRotator` (`SceneComponent.K2_GetComponentRotation` (`self.Camera_3D`))))
  (bind _returnvalue (- (`self.MaxZValue`) 0.0))
  (bind _returnvalue_2 (- (`self.MaxYValue`) 0.0))
  (bind (_returnvalue_roll_2 _returnvalue_pitch _returnvalue_yaw) (`KismetMathLibrary.BreakRotator` (`SceneComponent.K2_GetComponentRotation` (`/Game/ASST/Blueprints/Actors/Tracks/BP_Track.PlayerTracker` (`/Game/ASST/Blueprints/Characters/Player/BP_PlayerShip.CurrentTrack` (`self.PlayerRef`))))))
  ;[1 1 1] CUSTOM EVENTS
  (if (not (`/Game/ASST/Blueprints/Characters/Player/BP_PlayerShip.DoingSomersault?` (`self.PlayerRef`)))
    (`|ExecutionSequence`
      (:`then_0`
        (if (`self.ResetCameraRotation?`)
          (set `self.ResetCameraRotation?` false)
          (`SceneComponent.K2_SetRelativeRotation` (`self.Camera_3D`) (`KismetMathLibrary.MakeRotator` 0.0 (`self.CameraPitch`)) false false)))
      (:`then_1`
        (`self.K2_SetActorLocation` (`SplineComponent.GetLocationAtDistanceAlongSpline` (`/Game/ASST/Blueprints/Actors/Tracks/BP_Track.Spline` (`/Game/ASST/Blueprints/Characters/Player/BP_PlayerShip.CurrentTrack` _playerref)) (`/Game/ASST/Blueprints/Characters/Player/BP_PlayerShip.DistanceAlongTrack` _playerref) "World") false true)
        (switch `/Game/ASST/Enums/Enum_PerspectiveTypes` (`self.CurrentPerspective`)
          (:`NewEnumerator0`
            (set `self.CameraPercentOffset` 0.25))
          (:`NewEnumerator2`
            (`self.K2_SetActorRotation` (`KismetMathLibrary.MakeRotator` _returnvalue_roll _returnvalue_pitch _returnvalue_yaw) true)
            (set `self.CameraPercentOffset` 0.8)))
        (`SceneComponent.K2_SetRelativeLocation` (`self.Camera_3D`) (`KismetMathLibrary.MakeVector` 0.0 (`KismetMathLibrary.FClamp` (* (`/Game/ASST/Blueprints/Characters/Player/BP_PlayerShip.FTrackYOffset` _playerref_2) _camerapercentoffset) (* _returnvalue_2 -1.0) (* _returnvalue_2 1.0)) (+ (`KismetMathLibrary.FClamp` (* (`/Game/ASST/Blueprints/Characters/Player/BP_PlayerShip.FTrackZOffset` _playerref_2) _camerapercentoffset) (* _returnvalue -1.0) (* _returnvalue 1.0)) (`self.CameraZOffset`))) false true)))
    (else
      (`SceneComponent.K2_SetRelativeRotation` (`self.Camera_3D`) (`KismetMathLibrary.FindLookAtRotation` (`SceneComponent.K2_GetComponentLocation` (`self.Camera_3D`)) (`self.K2_GetActorLocation` (`self.PlayerRef`))) false false)
      (set `self.ResetCameraRotation?` true))))

(event `EventStageClear`
  (bind _playerref (`self.PlayerRef`))
  (bind _springarm_3d (`self.SpringArm_3D`))
  (bind _returnvalue (`self.K2_GetActorLocation` _playerref))
  ;[1 1 1] CUSTOM EVENTS
  (switch `/Game/ASST/Enums/Enum_PerspectiveTypes` (`/Game/ASST/Blueprints/Characters/Player/BP_PlayerShip.CurrentPerspective` (`self.PlayerRef`))
    (:`NewEnumerator2`
      (if (`/Game/ASST/Blueprints/Characters/Player/BP_PlayerShip.TrackModeActive` (`self.PlayerRef`))
        (`self.K2_SetActorLocation` _returnvalue false true)
        (else
          (`self.K2_SetActorLocationAndRotation` _returnvalue (`self.K2_GetActorRotation` _playerref) false true)))
      (if (`self.RotateCamera?`)
        (`/Engine/EditorBlueprintResources/StandardMacros.DoOnce` false
          (:`Completed`
            (`PlayerController.SetViewTargetWithBlend` (`GameplayStatics.GetPlayerController` 0) self 1.0 "VTBlend_Cubic" 0.0 false)
            (`SceneComponent.K2_SetRelativeLocation` (`self.Camera_3D`) (0.0 0.0 80.0) false true)
            (bind (_direction _alpha) (`Timeline|TM_RotateCamera`)
              (:`Update`
                (`SceneComponent.K2_SetRelativeRotation` (`self.SpringArm_3D`) (`KismetMathLibrary.MakeRotator` 0.0 0.0 (`KismetMathLibrary.Lerp` 0.0 240.0 _alpha)) false true)
                (set `SpringArmComponent.TargetArmLength` (+ (`SpringArmComponent.TargetArmLength` _springarm_3d) 0.5) _springarm_3d))
              (:`Finished`
                (`ActorComponent.SetActive` (`self.CameraFront`) true false)
                (`ActorComponent.SetActive` (`self.Camera_3D`) false false)
                (bind (_direction_2 _alpha_2) (`Timeline|TM_CloseUp`)
                  (:`Update`
                    (set `SpringArmComponent.TargetArmLength` (`KismetMathLibrary.Lerp` 300.0 450.0 _alpha_2) (`self.SpringArm1`))))))))))))

(event `EventCenterCamera`
  (bind _playerref (`self.PlayerRef`))
  ;[1 1 1] CUSTOM EVENTS
  (`SceneComponent.K2_SetRelativeLocationAndRotation` (`self.Camera_3D`) (`KismetMathLibrary.MakeVector` 0.0 0.0 (`self.CameraZOffset`)) (`KismetMathLibrary.MakeRotator` 0.0 (`self.CameraPitch`)) false true)
  (`self.K2_SetActorLocationAndRotation` (`self.K2_GetActorLocation` _playerref) (`self.K2_GetActorRotation` _playerref) false true))

(fn `RelativeSpringArm_CameraTransformOffset`
  (params (NewSpringArmRotation :type "Rotator Structure") (NewTargetArmLength :type "Float (double-precision)") (NewSpringArmLocation :type "Vector Structure") (NewCameraRotation :type "Rotator Structure"))
  (bind _springarm_3d (`self.SpringArm_3D`))
  (`SceneComponent.K2_SetRelativeRotation` _springarm_3d NewSpringArmRotation false false)
  (set `SpringArmComponent.TargetArmLength` NewTargetArmLength _springarm_3d)
  (`SceneComponent.K2_SetRelativeLocation` _springarm_3d NewSpringArmLocation false false)
  (`SceneComponent.K2_SetRelativeRotation` (`self.Camera_3D`) NewCameraRotation false false))

(fn `UserConstructionScript`)