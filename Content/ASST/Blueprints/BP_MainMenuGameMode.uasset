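; Game mode for the main menu that shows the menu widget and owns the player's save data.
; On BeginPlay it adds WBP_MainMenu with UI-only input, then loads the PlayerSave slot or creates and saves a new one, and pushes its stats to the HUD.
; SetLoadOut writes the chosen utility, two weapons and ship into the save and saves it immediately.
; A debug print shows the saved Overdrives count.
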(event `self.ReceiveBeginPlay`
  (bind _hud_ref (`self.HUD_Ref`))
  ;[1 1 1] Load Menu UI
  (bind _returnvalue (`|CreateWidget` "/Game/ASST/Blueprints/UMG/Menus/WBP_MainMenu.WBP_MainMenu_C"))
  (set `self.HUD_Ref` _returnvalue)
  (`UserWidget.AddToViewport` _hud_ref 0)
  (`WidgetBlueprintLibrary.SetInputMode_UIOnlyEx` (`GameplayStatics.GetPlayerController` 0) _hud_ref)
  ;[1 1 1] Does a save file exist?
  (bind _returnvalue_2 (`GameplayStatics.DoesSaveGameExist` "PlayerSave_00"))
  (if _returnvalue_2
    ;[1 1 1] Load PlayerSave
    (bind _ass_player_save (`/Game/ASST/Blueprints/Characters/Player/PlayerSave_Library.LoadPlayerSave` "PlayerSave_00"))
    (set `self.S_PlayerSave` _ass_player_save)
    (else
      ;[1 1 1] Create new PlayerSave
      (bind _returnvalue_3 (`/Game/ASST/Blueprints/Characters/Player/PlayerSave_Library.CreatePlayerSave`))
      (set `self.S_PlayerSave` _returnvalue_3)
      (`/Game/ASST/Blueprints/Characters/Player/PlayerSave_Library.SavePlayerSave` (`self.S_PlayerSave`) "PlayerSave_00")))
  ;[1 1 1] Update hud stats
  (`/Game/ASST/Blueprints/UMG/Menus/WBP_MainMenu.Update_HUDStats` (`self.HUD_Ref`) (`self.S_PlayerSave`))
  (`KismetSystemLibrary.PrintString` (`KismetStringLibrary.Concat_StrStr` "Overdrives Used: " (`KismetStringLibrary.Conv_IntToString` (`BlueprintMapLibrary.Map_Find` (`/Game/ASST/Blueprints/Actors/SaveGame/S_PlayerSave.Int_MiscStats` (`self.S_PlayerSave`)) "Overdrives"))) true true (struct :`R` 0.972124 :`B` 1.0 :`A` 1.0)))

(fn `SetLoadOut`
  (params (Utility :type "/Game/ASST/Blueprints/Actors/Weapons/Player/Utilities/BP_Utility Class Reference") (Weapon1 :type "/Game/ASST/Blueprints/Actors/Weapons/Player/Weapons/BP_WepBase Class Reference") (Weapon2 :type "/Game/ASST/Blueprints/Actors/Weapons/Player/Weapons/BP_WepBase Class Reference") (PlayerShip :type "/Game/ASST/Blueprints/Characters/Player/BP_PlayerShip Class Reference"))
  (bind _s_playersave (`self.S_PlayerSave`))
  (set `/Game/ASST/Blueprints/Actors/SaveGame/S_PlayerSave.Utility` Utility _s_playersave)
  (set `/Game/ASST/Blueprints/Actors/SaveGame/S_PlayerSave.Weapon1` Weapon1 _s_playersave)
  (set `/Game/ASST/Blueprints/Actors/SaveGame/S_PlayerSave.Weapon2` Weapon2 _s_playersave)
  (set `/Game/ASST/Blueprints/Actors/SaveGame/S_PlayerSave.PlayerShip` PlayerShip _s_playersave)
  (`/Game/ASST/Blueprints/Characters/Player/PlayerSave_Library.SavePlayerSave` (`self.S_PlayerSave`) "PlayerSave_00"))

(fn `UserConstructionScript`)