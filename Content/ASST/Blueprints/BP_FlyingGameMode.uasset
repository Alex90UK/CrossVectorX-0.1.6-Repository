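; BP_FlyingGameMode is the game mode for flying gameplay and drives level initialization at BeginPlay.
; It calls InitMessage on the first player controller, then InitChain forwards the same message to every BP_Track, BP_FixedCameraActor and BP_StageClear actor, in that order.
; It then spawns an EventManager that it owns and stores the reference, so startup order is set centrally.
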(event `self.ReceiveBeginPlay`
  (message `/Game/ASST/Blueprints/Characters/Player/ISetup.Init` (`GameplayStatics.GetPlayerController` 0))
  (`self.InitChain`)
  ;[1 1 1] Spawn event manager
  (bind _returnvalue (`|SpawnActorFromClass` "/Game/ASST/Blueprints/Actors/Combo/EventManager.EventManager_C" (`KismetMathLibrary.MakeTransform` (0.0 0.0 0.0)) "AlwaysSpawn" "OverrideRootScale" self null))
  (set `self.EventManager` _returnvalue))

(fn `InitChain`
  (bind _outactors (`GameplayStatics.GetAllActorsOfClass` "/Game/ASST/Blueprints/Actors/Tracks/BP_Track.BP_Track_C"))
  (for _array_element _outactors
    (message `/Game/ASST/Blueprints/Characters/Player/ISetup.Init` _array_element))
  (bind _outactors_2 (`GameplayStatics.GetAllActorsOfClass` "/Game/ASST/Blueprints/Actors/Camera/BP_FixedCameraActor.BP_FixedCameraActor_C"))
  (for _array_element_2 _outactors_2
    (message `/Game/ASST/Blueprints/Characters/Player/ISetup.Init` _array_element_2))
  (bind _outactors_3 (`GameplayStatics.GetAllActorsOfClass` "/Game/ASST/Blueprints/Actors/Tools/BP_StageClear.BP_StageClear_C"))
  (for _array_element_3 _outactors_3
    (message `/Game/ASST/Blueprints/Characters/Player/ISetup.Init` _array_element_3)))

(fn `UserConstructionScript`)