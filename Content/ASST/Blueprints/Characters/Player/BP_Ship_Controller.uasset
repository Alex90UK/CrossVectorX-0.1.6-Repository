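; Player controller for the ship that handles spawning, weapons, score, multiplier and overdrive.
; Init loads the save, spawns and possesses the chosen ship at a PlayerStart, and builds its loadout, with defaults if no save exists.
; Score, multiplier and loadout components do the work; the controller relays changes through dispatchers and sets loadout level from the multiplier.
; It records stage-clear and overdrive stats, and includes debug keys and on-screen readouts.
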(event `Event_StageCleared`
  ;[1 1 1] Stage cleared
  (`/Game/ASST/Blueprints/Characters/Player/PlayerSave_Library.Update_PlayerStat` (`self.S_PlayerSave`) "AccumilatedScore" (`/Game/ASST/Blueprints/Characters/Player/C_Score.Score` (`self.C_Score`)))
  (`/Game/ASST/Blueprints/Characters/Player/PlayerSave_Library.Update_PlayerStat` (`self.S_PlayerSave`) "MissionsCompleted" 1))

(event `Key|One`
  (params (Key :type "Key Structure"))
  ;[1 1 1] Testing (Debugs)
  (:`Pressed`
    (`/Game/ASST/Blueprints/Characters/Player/C_MultiplierManager.ModifyMultiplierProgression` (`self.C_MultiplierManager`) true 50)
    (`self.MultiplierProgressionChanged` :!label _label)))

(event `self.ReceiveTick`
  (params (DeltaSeconds :type "Float (single-precision)"))
  (bind _c_multipliermanager (`self.C_MultiplierManager`))
  ;[1 1 1] Testing (Debugs)
  (`KismetSystemLibrary.Delay` 1.0)
  (`|ExecutionSequence`
    (:`then_0`
      (`KismetSystemLibrary.PrintString` (`KismetStringLibrary.Concat_StrStr` "Multiplier: " (`KismetStringLibrary.Conv_IntToString` (`/Game/ASST/Blueprints/Characters/Player/C_MultiplierManager.Multiplier` _c_multipliermanager)) "  Progression:  " (`KismetStringLibrary.Conv_IntToString` (`/Game/ASST/Blueprints/Characters/Player/C_MultiplierManager.ProgressionAmount` _c_multipliermanager)) " Scaler: " (`KismetStringLibrary.Conv_IntToString` (`/Game/ASST/Blueprints/Characters/Player/C_MultiplierManager.MultiplierScaler` _c_multipliermanager))) true true (struct :`R` 0.541667 :`B` 0.347457 :`A` 1.0) 1.0))
    (:`then_1`
      (`KismetSystemLibrary.PrintString` (`KismetStringLibrary.Concat_StrStr` "Overdrive: " (`KismetStringLibrary.Conv_IntToString` (`/Game/ASST/Blueprints/Characters/Player/C_MultiplierManager.Overdrive` _c_multipliermanager)) " IsActive: " (`KismetStringLibrary.Conv_BoolToString` (`/Game/ASST/Blueprints/Characters/Player/C_MultiplierManager.IsOverdriveActive` _c_multipliermanager))) true true (struct :`R` 0.875 :`G` 0.756765 :`A` 1.0) 1.0))
    (:`then_2`
      (`KismetSystemLibrary.PrintString` (`KismetStringLibrary.Concat_StrStr` "SCORE: " (`KismetStringLibrary.Conv_IntToString` (`/Game/ASST/Blueprints/Characters/Player/C_Score.Score` (`self.C_Score`)))) true true (struct :`R` 0.875 :`G` 0.325167 :`A` 1.0) 1.0))))

(event `/Game/ASST/Blueprints/Characters/Player/IController.ModifyMultiplierProgression`
  (params (IsPositive :type Boolean) (InAmount :type Integer))
  ;[1 1 1] Score, overdrive and multipliers
  ;;[1 1 1] Modify Multiplier progression
  (`/Game/ASST/Blueprints/Characters/Player/C_MultiplierManager.ModifyMultiplierProgression` (`self.C_MultiplierManager`) IsPositive InAmount)
  (`self.MultiplierProgressionChanged`))

(event `/Game/ASST/Blueprints/Characters/Player/IController.ActivateOverdrive`
  ;[1 1 1] Score, overdrive and multipliers
  ;;[1 1 1] Activate/deactivate Overdrive
  (`/Game/ASST/Blueprints/Characters/Player/C_MultiplierManager.ActivateOverdrive` (`self.C_MultiplierManager`)))

(event `Key|Two`
  (params (Key :type "Key Structure"))
  ;[1 1 1] Testing (Debugs)
  (:`Pressed`
    (`/Game/ASST/Blueprints/Characters/Player/C_MultiplierManager.ModifyMultiplierProgression` (`self.C_MultiplierManager`) false 25)
    (goto _label)))

(event `/Game/ASST/Blueprints/Characters/Player/IController.ModifyScore`
  (params (IsPositive :type Boolean) (InAmount :type Integer))
  ;[1 1 1] Score, overdrive and multipliers
  ;;[1 1 1] Modify Score
  (`/Game/ASST/Blueprints/Characters/Player/C_Score.ModifyScore` (`self.C_Score`) IsPositive InAmount (`/Game/ASST/Blueprints/Characters/Player/C_MultiplierManager.Multiplier` (`self.C_MultiplierManager`)))
  (`self.ScoreChanged`))

(event `Key|Three`
  (params (Key :type "Key Structure"))
  (bind _c_multipliermanager (`self.C_MultiplierManager`))
  ;[1 1 1] Testing (Debugs)
  (:`Pressed`
    (`/Game/ASST/Blueprints/Characters/Player/C_MultiplierManager.ActivateOverdrive` _c_multipliermanager)
    (`self.OverdriveActivated`)
    (add `/Game/ASST/Blueprints/Characters/Player/C_MultiplierManager.EDeactivateOverdrive` _c_multipliermanager (delegate `ETEST`))
    (`self.MultiplierProgressionChanged` :!label _label_2)))

(event `/Game/ASST/Blueprints/Characters/Player/IController.ModifyOverdriveProgression`
  (params (IsPositive :type Boolean) (InAmount :type Integer))
  ;[1 1 1] Score, overdrive and multipliers
  ;;[1 1 1] Modify Overdrive Progrssion
  (`/Game/ASST/Blueprints/Characters/Player/C_MultiplierManager.Modify OverdriveProgression` (`self.C_MultiplierManager`) IsPositive InAmount)
  (`self.OverdriveProgressionChanged`))

(event `ETEST`
  ;[1 1 1] Testing (Debugs)
  (`self.Overdrivedeactivated`)
  (goto _label_2))

(event `Key|Four`
  (params (Key :type "Key Structure"))
  ;[1 1 1] Testing (Debugs)
  (:`Pressed`
    (`/Game/ASST/Blueprints/Characters/Player/C_MultiplierManager.Modify OverdriveProgression` (`self.C_MultiplierManager`) true 50)
    (`self.OverdriveProgressionChanged`)))

(event `self.ReceiveBeginPlay`)

(event `/Game/ASST/Blueprints/Characters/Player/ISetup.Init`
  ;[1 1 1] load save
  (`self.LoadSave`)
  ;[1 1 1] Spawn players ship
  (`self.SpawnCharacter`)
  ;[1 1 1] WEAPONS
  ;;[0.7812 0 0.01819] Call from set up later on with init setup
  (`/Engine/EditorBlueprintResources/StandardMacros.IsValid` (`self.S_PlayerSave`)
    (:`Is Valid`
      (bind (_utility _weapon1 _weapon2 _passive) (`/Game/ASST/Blueprints/Characters/Player/PlayerSave_Library.Get_SavedLoadout` (`self.S_PlayerSave`)))
      (`/Game/ASST/Blueprints/Characters/Player/C_Loadout.CreateLoadout` (`self.C_Loadout`) _utility _weapon1 _weapon2 _passive))
    (:`Is Not Valid`
      (`/Game/ASST/Blueprints/Characters/Player/C_Loadout.CreateLoadout` (`self.C_Loadout`) "/Game/ASST/Blueprints/Actors/Weapons/Player/Utilities/U_Somersault.U_Somersault_C" "/Game/ASST/Blueprints/Actors/Weapons/Player/Weapons/W_Laser.W_Laser_C" "/Game/ASST/Blueprints/Actors/Weapons/Player/Weapons/W_ChargeLaser.W_ChargeLaser_C" null)))
  ;;[1 1 1] Multiplier changed
  (add `/Game/ASST/Blueprints/Characters/Player/C_MultiplierManager.EMultiplierChanged` (`self.C_MultiplierManager`) (delegate `EMultiplierChanged`))
  ;;[1 1 1] OverdriveDeactivated
  (add `/Game/ASST/Blueprints/Characters/Player/C_MultiplierManager.EDeactivateOverdrive` (`self.C_MultiplierManager`) (delegate `DeactivatedOverdrive`))
  (`self.MultiplierProgressionChanged` :!label _label_3)
  ;;[1 1 1] OverdriveActivated Event
  (add `/Game/ASST/Blueprints/Characters/Player/C_MultiplierManager.EOverdriveActivated` (`self.C_MultiplierManager`) (delegate `EOverdriveActivated`)))

(event `Key|Five`
  (params (Key :type "Key Structure"))
  ;[1 1 1] Testing (Debugs)
  (:`Pressed`
    (`/Game/ASST/Blueprints/Characters/Player/C_Score.ModifyScore` (`self.C_Score`) true 25 (`/Game/ASST/Blueprints/Characters/Player/C_MultiplierManager.Multiplier` (`self.C_MultiplierManager`)))
    (`self.ScoreChanged`)))

(event `EMultiplierChanged`
  ;[1 1 1] WEAPONS
  ;;[1 1 1] Multiplier changed
  (`self.MultiplierChanged`)
  (`/Game/ASST/Blueprints/Actors/Weapons/IWeapons.ModifyLoadoutLevel` self (`/Game/ASST/Blueprints/Characters/Player/C_MultiplierManager.Multiplier` (`self.C_MultiplierManager`))))

(event `DeactivatedOverdrive`
  ;[1 1 1] WEAPONS
  ;;[1 1 1] OverdriveDeactivated
  (`self.Overdrivedeactivated`)
  (goto _label_3))

(event `EOverdriveActivated`
  (bind _s_playersave (`self.S_PlayerSave`))
  ;[1 1 1] WEAPONS
  ;;[1 1 1] OverdriveActivated Event
  (`self.OverdriveActivated`)
  (`/Engine/EditorBlueprintResources/StandardMacros.IsValid` _s_playersave
    (:`Is Valid`
      ;[1 1 1] Update Stat
      (`/Game/ASST/Blueprints/Characters/Player/PlayerSave_Library.Update_PlayerStat` _s_playersave "Overdrives" 1))))

(event `/Game/ASST/Blueprints/Actors/Weapons/IWeapons.UseUtility`
  ;[1 1 1] WEAPONS
  ;;[1 1 1] Shooting weapons
  (`/Game/ASST/Blueprints/Characters/Player/C_Loadout.FireUtility` (`self.C_Loadout`)))

(event `/Game/ASST/Blueprints/Actors/Weapons/IWeapons.UseWeapon1`
  ;[1 1 1] WEAPONS
  ;;[1 1 1] Shooting weapons
  (`/Game/ASST/Blueprints/Characters/Player/C_Loadout.FireWeapon1` (`self.C_Loadout`)))

(event `/Game/ASST/Blueprints/Actors/Weapons/IWeapons.StopWeapon1`
  ;[1 1 1] WEAPONS
  ;;[1 1 1] Shooting weapons
  (`/Game/ASST/Blueprints/Characters/Player/C_Loadout.StopFiring1` (`self.C_Loadout`)))

(event `/Game/ASST/Blueprints/Actors/Weapons/IWeapons.UsePassive`
  ;[1 1 1] WEAPONS
  ;;[1 1 1] Shooting weapons
  (`/Game/ASST/Blueprints/Characters/Player/C_Loadout.UsePassive` (`self.C_Loadout`)))

(event `/Game/ASST/Blueprints/Actors/Weapons/IWeapons.UseWeapon2`
  ;[1 1 1] WEAPONS
  ;;[1 1 1] Shooting weapons
  (`/Game/ASST/Blueprints/Characters/Player/C_Loadout.FireWeapon2` (`self.C_Loadout`)))

(event `/Game/ASST/Blueprints/Actors/Weapons/IWeapons.StopWeapon2`
  ;[1 1 1] WEAPONS
  ;;[1 1 1] Shooting weapons
  (`/Game/ASST/Blueprints/Characters/Player/C_Loadout.StopFiring2` (`self.C_Loadout`)))

(event `/Game/ASST/Blueprints/Actors/Weapons/IWeapons.ModifyLoadoutLevel`
  (params (Level :type Integer))
  ;[1 1 1] WEAPONS
  ;;[1 1 1] Shooting weapons
  (`/Game/ASST/Blueprints/Characters/Player/C_Loadout.ModifyLoadoutLevels` (`self.C_Loadout`) Level))

(fn `LoadSave`
  (bind _returnvalue (`GameplayStatics.DoesSaveGameExist` "PlayerSave_00"))
  (if _returnvalue
    (bind _ass_player_save (`/Game/ASST/Blueprints/Characters/Player/PlayerSave_Library.LoadPlayerSave` "PlayerSave_00"))
    (set `self.S_PlayerSave` _ass_player_save)))

(fn `SpawnCharacter`
  (bind _s_playersave (`self.S_PlayerSave`))
  (bind _shipclass (`self.ShipClass`))
  (`/Engine/EditorBlueprintResources/StandardMacros.IsValid` _s_playersave
    (:`Is Valid`
      (set `self.ShipClass` (`/Game/ASST/Blueprints/Actors/SaveGame/S_PlayerSave.PlayerShip` _s_playersave)))
    (:`Is Not Valid`
      (set `self.ShipClass` "/Game/ASST/Blueprints/Characters/Player/BP_PlayerShip.BP_PlayerShip_C")))
  (bind _outactors (`GameplayStatics.GetAllActorsOfClass` "/Script/Engine.PlayerStart"))
  (bind _output (`|GetArrayItem` _outactors))
  (`/Engine/EditorBlueprintResources/StandardMacros.IsValid` _output
    (:`Is Valid`
      (bind _returnvalue (`|SpawnActorFromClass` _shipclass (`KismetMathLibrary.MakeTransform` (`self.K2_GetActorLocation` _output)) "AlwaysSpawn" "OverrideRootScale" null null))
      (`self.Possess` self _returnvalue))
    (:`Is Not Valid`
      (bind _returnvalue_2 (`|SpawnActorFromClass` _shipclass (`KismetMathLibrary.MakeTransform` (0.0 0.0 0.0)) "AlwaysSpawn" "OverrideRootScale" null null))
      (`self.Possess` self _returnvalue_2))))

(fn `UserConstructionScript`)