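; Venom flying enemy, a child Blueprint that sets its avoidance radius and death delay and removes its exhaust when destroyed.
; On fire, it maps damage type to a projectile tag, then, for the Laser weapon, spawns tagged lasers from left and right points aimed at the player.
; Projectile type can make each laser home on the player ship or trigger its never-miss event.
; Fireball spawning logic exists but is disconnected.
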(event `self.ReceiveBeginPlay`
  (`parent.ReceiveBeginPlay`)
  ;[1 1 1] Collision radius used for obstacle avoidance
  (set `self.CollisionSphereRadius` 100.0))

(event `self.EventFire`
  (bind _returnvalue (`SceneComponent.K2_GetComponentLocation` (`self.SpawnPointRight`)))
  (bind _returnvalue_2 (`SceneComponent.K2_GetComponentLocation` (`self.SpawnPointLeft`)))
  ;[1 1 1] CUSTOM EVENTS
  (switch `/Game/ASST/Enums/Enum_DamageType` (`self.DamageType`)
    (:`NewEnumerator0`
      (set `self.ProjectileTag` (`self.CrashTag`)))
    (:`NewEnumerator1`
      (set `self.ProjectileTag` (`self.LightTag`)))
    (:`NewEnumerator2`
      (set `self.ProjectileTag` (`self.HeavyTag`)))
    (:`NewEnumerator3`
      (set `self.ProjectileTag` (`self.ShieldBreakTag`)))
    (:`NewEnumerator4`
      (set `self.ProjectileTag` (`self.InstaDeathTag`))))
  (switch `/Game/ASST/Enums/Enum_WeaponType` (`self.WeaponType`)
    (:`NewEnumerator0`
      (`|ExecutionSequence`
        (:`then_0`
          (bind _returnvalue_3 (`|SpawnActorFromClass` "/Game/ASST/Blueprints/Actors/Weapons/EnemyWeapons/BP_EnemyLaser.BP_EnemyLaser_C" (`KismetMathLibrary.MakeTransform` (+ _returnvalue_2 (100.0 0.0 0.0)) (`KismetMathLibrary.FindLookAtRotation` _returnvalue_2 (`SceneComponent.K2_GetComponentLocation` (`Actor.RootComponent` (`self.PlayerRef`)))) (4.0 4.0 4.0)) "AlwaysSpawn" "OverrideRootScale" null null))
          (set `Actor.Tags` (`self.ProjectileTag`) _returnvalue_3)
          (switch `/Game/ASST/Enums/Enum_EnemyProjectileType` (`self.ProjectileType`)
            (:`NewEnumerator1`
              (bind _asbp_player_ship (cast `/Game/ASST/Blueprints/Characters/Player/BP_PlayerShip` (`GameplayStatics.GetPlayerPawn` 0)))
              (bind _projectilemovement (`/Game/ASST/Blueprints/Actors/Weapons/EnemyWeapons/BP_EnemyLaser.ProjectileMovement` _returnvalue_3))
              (set `ProjectileMovementComponent.HomingTargetComponent` (`/Game/ASST/Blueprints/Characters/Player/BP_PlayerShip.Root` _asbp_player_ship) _projectilemovement)
              (set `ProjectileMovementComponent.bIsHomingProjectile` true _projectilemovement)
              (set `ProjectileMovementComponent.HomingAccelerationMagnitude` 40000.0 _projectilemovement))
            (:`NewEnumerator2`
              (`/Game/ASST/Blueprints/Actors/Weapons/EnemyWeapons/BP_EnemyLaser.EventNeverMiss` _returnvalue_3 (`GameplayStatics.GetPlayerPawn` 0)))))
        (:`then_1`
          (bind _returnvalue_4 (`|SpawnActorFromClass` "/Game/ASST/Blueprints/Actors/Weapons/EnemyWeapons/BP_EnemyLaser.BP_EnemyLaser_C" (`KismetMathLibrary.MakeTransform` (+ _returnvalue (100.0 0.0 0.0)) (`KismetMathLibrary.FindLookAtRotation` _returnvalue (`SceneComponent.K2_GetComponentLocation` (`/Game/ASST/Blueprints/Characters/Player/BP_PlayerShip.Root` (`self.PlayerRef`)))) (4.0 4.0 4.0)) "AlwaysSpawn" "OverrideRootScale" null null))
          (set `Actor.Tags` (`self.ProjectileTag`) _returnvalue_4)
          (switch `/Game/ASST/Enums/Enum_EnemyProjectileType` (`self.ProjectileType`)
            (:`NewEnumerator1`
              (bind _asbp_player_ship_2 (cast `/Game/ASST/Blueprints/Characters/Player/BP_PlayerShip` (`GameplayStatics.GetPlayerPawn` 0)))
              (bind _projectilemovement_2 (`/Game/ASST/Blueprints/Actors/Weapons/EnemyWeapons/BP_EnemyLaser.ProjectileMovement` _returnvalue_4))
              (set `ProjectileMovementComponent.HomingTargetComponent` (`/Game/ASST/Blueprints/Characters/Player/BP_PlayerShip.Root` _asbp_player_ship_2) _projectilemovement_2)
              (set `ProjectileMovementComponent.bIsHomingProjectile` true _projectilemovement_2)
              (set `ProjectileMovementComponent.HomingAccelerationMagnitude` 40000.0 _projectilemovement_2))
            (:`NewEnumerator2`
              (`/Game/ASST/Blueprints/Actors/Weapons/EnemyWeapons/BP_EnemyLaser.EventNeverMiss` _returnvalue_4 (`GameplayStatics.GetPlayerPawn` 0)))))))))

(event `self.EventDestroyed`
  (bind _p_exhaust (`self.P_Exhaust`))
  ;[1 1 1] CUSTOM EVENTS
  (set `self.Destroyed` true)
  (`/Engine/EditorBlueprintResources/StandardMacros.IsValid` _p_exhaust
    (:`Is Valid`
      (`ActorComponent.K2_DestroyComponent` _p_exhaust))))

(fn `UserConstructionScript`
  (`parent.UserConstructionScript`)
  ;[1 1 1] Set DM_DeathDelay to 10 - default in parentBP class
  (set `self.DM_DeathDelay` 10.0))