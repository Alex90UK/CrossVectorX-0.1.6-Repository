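; Flying enemy carrier ship that can carry three turrets, built on a parent enemy class with a larger avoidance radius and a longer death delay.
; On BeginPlay, if SpawnTurrets is set, it spawns BP_BasicTurret actors attached to top, left and right ship sockets, passing on tags and weapon settings.
; On destruction it removes exhaust particles and destroys those turrets so none are left floating.
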(event `self.ReceiveBeginPlay`
  (bind _topturret (`self.TopTurret`))
  (bind _leftturret (`self.LeftTurret`))
  (bind _rightturret (`self.RightTurret`))
  (`parent.ReceiveBeginPlay`)
  ;[1 1 1] Collision radius used for obstacle avoidance
  (set `self.CollisionSphereRadius` 6500.0)
  (if (`self.SpawnTurrets?`)
    ;[1 1 1] SPAWN TURRETS
    (`|ExecutionSequence`
      (:`then_0`
        (bind _returnvalue (`|SpawnActorFromClass` "/Game/ASST/Blueprints/Characters/Enemies/GroundEnemies/BP_BasicTurret.BP_BasicTurret_C" (`KismetMathLibrary.MakeTransform` (`SceneComponent.GetSocketLocation` (`self.Ship`) "TurretSocketTop")) "Undefined" "OverrideRootScale" null null))
        (bind _output_get (set `self.TopTurret` _returnvalue))
        (`self.K2_AttachToActor` _output_get self "TurretSocketTop" "KeepWorld" "KeepWorld" "KeepWorld" true)
        (set `Actor.Tags` (`self.TurretTags`) (`self.TopTurret`))
        (set `/Game/ASST/Blueprints/Characters/Enemies/GroundEnemies/BP_BasicTurret.WeaponType` (`self.TurretWeaponType`) _topturret)
        (set `/Game/ASST/Blueprints/Characters/Enemies/GroundEnemies/BP_BasicTurret.ProjectileType` (`self.TurretProjectileType`) _topturret)
        (set `/Game/ASST/Blueprints/Characters/Enemies/GroundEnemies/BP_BasicTurret.DamageType` (`self.TurretDamageType`) _topturret)
        (set `/Game/ASST/Blueprints/Characters/Enemies/GroundEnemies/BP_BasicTurret.FireRate` (`self.TurretFireRate`) _topturret))
      (:`then_1`
        (bind _returnvalue_2 (`|SpawnActorFromClass` "/Game/ASST/Blueprints/Characters/Enemies/GroundEnemies/BP_BasicTurret.BP_BasicTurret_C" (`KismetMathLibrary.MakeTransform` (`SceneComponent.GetSocketLocation` (`self.Ship`) "TurretSocketLeft")) "Undefined" "OverrideRootScale" null null))
        (bind _output_get_2 (set `self.LeftTurret` _returnvalue_2))
        (`self.K2_AttachToActor` _output_get_2 self "TurretSocketLeft" "KeepWorld" "KeepWorld" "KeepWorld" true)
        (set `Actor.Tags` (`self.TurretTags`) (`self.LeftTurret`))
        (set `/Game/ASST/Blueprints/Characters/Enemies/GroundEnemies/BP_BasicTurret.WeaponType` (`self.TurretWeaponType`) _leftturret)
        (set `/Game/ASST/Blueprints/Characters/Enemies/GroundEnemies/BP_BasicTurret.ProjectileType` (`self.TurretProjectileType`) _leftturret)
        (set `/Game/ASST/Blueprints/Characters/Enemies/GroundEnemies/BP_BasicTurret.DamageType` (`self.TurretDamageType`) _leftturret)
        (set `/Game/ASST/Blueprints/Characters/Enemies/GroundEnemies/BP_BasicTurret.FireRate` (`self.TurretFireRate`) _leftturret))
      (:`then_2`
        (bind _returnvalue_3 (`|SpawnActorFromClass` "/Game/ASST/Blueprints/Characters/Enemies/GroundEnemies/BP_BasicTurret.BP_BasicTurret_C" (`KismetMathLibrary.MakeTransform` (`SceneComponent.GetSocketLocation` (`self.Ship`) "TurretSocketRight")) "Undefined" "OverrideRootScale" null null))
        (bind _output_get_3 (set `self.RightTurret` _returnvalue_3))
        (`self.K2_AttachToActor` _output_get_3 self "TurretSocketRight" "KeepWorld" "KeepWorld" "KeepWorld" true)
        (set `Actor.Tags` (`self.TurretTags`) (`self.RightTurret`))
        (set `/Game/ASST/Blueprints/Characters/Enemies/GroundEnemies/BP_BasicTurret.WeaponType` (`self.TurretWeaponType`) _rightturret)
        (set `/Game/ASST/Blueprints/Characters/Enemies/GroundEnemies/BP_BasicTurret.ProjectileType` (`self.TurretProjectileType`) _rightturret)
        (set `/Game/ASST/Blueprints/Characters/Enemies/GroundEnemies/BP_BasicTurret.DamageType` (`self.TurretDamageType`) _rightturret)
        (set `/Game/ASST/Blueprints/Characters/Enemies/GroundEnemies/BP_BasicTurret.FireRate` (`self.TurretFireRate`) _rightturret)))))

(event `self.EventDestroyed`
  ;[1 1 1] CUSTOM EVENTS
  (set `self.Destroyed` true)
  (`ActorComponent.K2_DestroyComponent` (`self.P_Exhaust`))
  (`ActorComponent.K2_DestroyComponent` (`self.P_ExhaustLeft`))
  (`ActorComponent.K2_DestroyComponent` (`self.P_ExhaustRight`))
  (if (`self.SpawnTurrets?`)
    (`|ExecutionSequence`
      (:`then_0`
        (`self.K2_DestroyActor` (`self.TopTurret`)))
      (:`then_1`
        (`self.K2_DestroyActor` (`self.LeftTurret`)))
      (:`then_2`
        (`self.K2_DestroyActor` (`self.RightTurret`))))))

(fn `UserConstructionScript`
  (`parent.UserConstructionScript`)
  ;[1 1 1] Set DM_DeathDelay to 10 - default in parentBP class
  (set `self.DM_DeathDelay` 10.0))